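; BP_TetrisPlayerController is the player controller that turns Enhanced Input actions into Tetris piece commands.
; On BeginPlay it adds the IM_Context mapping context.
; IA_Space prints the action's name and calls RotatePiece, while IA_Move calls MoveRight, MoveLeft or MoveDown by axis sign, with horizontal input taking priority.
; The movement and rotation functions are only called here, not defined in its graphs.
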(event `self.ReceiveBeginPlay`
  (`EnhancedInputSubsystemInterface.AddMappingContext` (pcsubsystem `EnhancedInputLocalPlayerSubsystem` self) "/Game/Input/IM_Context.IM_Context" 0 (struct)))

(event `EnhancedInput|/Game/Input/IA_Space`
  (params (ActionValue :type Boolean) (ElapsedSeconds :type "Float (double-precision)") (TriggeredSeconds :type "Float (double-precision)") (InputAction :type "InputAction Object Reference" :default "/Game/Input/IA_Space.IA_Space"))
  (:`Triggered`
    (`KismetSystemLibrary.PrintString` (`KismetSystemLibrary.GetDisplayName` InputAction))
    (`self.RotatePiece`)))

(event `EnhancedInput|/Game/Input/IA_Move`
  (params (ActionValue :type "Vector2D Structure") (ElapsedSeconds :type "Float (double-precision)") (TriggeredSeconds :type "Float (double-precision)") (InputAction :type "InputAction Object Reference" :default "/Game/Input/IA_Move.IA_Move"))
  (bind (_x _y) (`KismetMathLibrary.BreakVector2D` ActionValue))
  (:`Triggered`
    (if (> _x 0.0)
      (`self.MoveRight`)
      (elif (< _x 0.0)
        (`self.MoveLeft`)
        (elif (< _y 0.0)
          (`self.MoveDown`))))))

(fn `UserConstructionScript`)