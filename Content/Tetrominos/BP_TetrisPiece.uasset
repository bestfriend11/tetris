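; BP_TetrisPiece is a falling tetromino that descends on a looping timer until it lands.
; On BeginPlay it collects static mesh children tagged "Piece" into Blocks and starts the fall timer.
; Each tick of that timer line-traces below every root child component for WorldStatic objects.
; A first hit clears the timer through a DoOnce; otherwise the piece calls Move to step down.
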(event `self.ReceiveBeginPlay`
  (`self.InitPieces`)
  (bind _returnvalue (`KismetSystemLibrary.K2_SetTimerDelegate` (delegate `FallingBlock`) (`self.Time`) true))
  (set `self.FallingTimerHandler` _returnvalue))

(event `FallingBlock`
  (set `self.ShouldFall` true)
  (for _array_element (`SceneComponent.GetChildrenComponents` (`self.DefaultSceneRoot`) false)
    (bind _returnvalue (`SceneComponent.K2_GetComponentLocation` _array_element))
    (bind (_outhit _returnvalue_2) (`KismetSystemLibrary.LineTraceSingleForObjects` :`Start` (+ _returnvalue (0.0 0.0 -50.0)) :`End` (- _returnvalue (0.0 0.0 100.0)) :`ObjectTypes` (`|MakeArray` "ObjectTypeQuery1" :!type "EObjectTypeQuery Enum") :`DrawTime` 1.0))
    (if _returnvalue_2
      (`/Engine/EditorBlueprintResources/StandardMacros.DoOnce` false
        (:`Completed`
          (set `self.ShouldFall` false)
          (`KismetSystemLibrary.K2_ClearAndInvalidateTimerHandle` (`self.FallingTimerHandler`))))))
  (if (`self.ShouldFall`)
    (`self.Move` (0.0 0.0 -0.5))))

(fn `InitPieces`
  (for _array_element (`SceneComponent.GetChildrenComponents` (`self.DefaultSceneRoot`) false)
    (bind _asstatic_mesh_component (cast `StaticMeshComponent` _array_element))
    (if (`ActorComponent.ComponentHasTag` _asstatic_mesh_component "Piece")
      (`KismetArrayLibrary.Array_Add` (`self.Blocks`) _asstatic_mesh_component))))

(fn `UserConstructionScript`)