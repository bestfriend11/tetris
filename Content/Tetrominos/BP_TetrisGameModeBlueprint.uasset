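; Tetris game mode Blueprint that starts a match and tracks score and level.
; On BeginPlay it resets score and level, then after a short delay asks the player controller's game board to spawn a piece.
; AddScore awards level-scaled points for cleared lines, raises the level when score passes a level-based threshold, and broadcasts both through a score-changed dispatcher.
; GameOver is an empty stub.
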(event `self.ReceiveBeginPlay`
  (set `self.Score` 0)
  (set `self.Level` 1)
  (`KismetSystemLibrary.Delay` 0.2)
  (`self.SpawnNewPiece`))

(fn `AddScore`
  (params (LinesCleared :type Integer :default 1))
  (bind _output_get (set `self.Score` (+ (`self.Score`) (* (`self.Level`) (select `int` LinesCleared :`0` 0 :`1` 100 :`2` 300 :`3` 500 :`4` 800)))))
  (`|ExecutionSequence`
    (:`then_0`
      (if (> _output_get (* 1000 (`self.Level`)))
        (`/Engine/EditorBlueprintResources/StandardMacros.IncrementInt` (`self.Level`))))
    (:`then_1`
      (`self.OnScoreChanged` (`self.Level`) (`self.Score`)))))

(fn `GameOver`)

(fn `SpawnNewPiece`
  (bind _asbp_tetris_player_controller (cast `/TetrisGame/Tetrominos/BP_TetrisPlayerController` (`GameplayStatics.GetPlayerController` 0)))
  (set `self.TetrisPlayerController` _asbp_tetris_player_controller)
  (bind _tetrisplayercontroller (`self.TetrisPlayerController`)
    (:`then`
      (`TetrisBoard.SpawnNewPiece` (`TetrisPlayerController.GetGameBoard` _tetrisplayercontroller)))
    (:`else`)))

(fn `UserConstructionScript`)